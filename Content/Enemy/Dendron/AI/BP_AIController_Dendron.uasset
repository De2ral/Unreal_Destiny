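; AI controller for the Dendron enemy that flags whether its target is close enough to attack.
; Tick passes through a one-second Delay, so the check runs roughly once per second.
; It reads the target actor from the Blackboard, measures its distance to the controlled pawn against a fixed range, and writes the result to the Atk key.
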(event `self.ReceiveTick`
  (params (DeltaSeconds :type "Float (single-precision)"))
  (bind _returnvalue (`AIBlueprintHelperLibrary.GetBlackboard` null))
  (bind _atk (`self.atk`))
  (`KismetSystemLibrary.Delay` 1.0)
  (bind `_as액터` (cast `Actor` (`BlackboardComponent.GetValueAsObject` _returnvalue (`self.targegt`))))
  (if (< (`KismetMathLibrary.Vector_Distance` (`self.K2_GetActorLocation` (`self.K2_GetPawn`)) (`self.K2_GetActorLocation` `_as액터`)) 4000.0)
    (`BlackboardComponent.SetValueAsBool` _returnvalue _atk true)
    (else
      (`BlackboardComponent.SetValueAsBool` _returnvalue _atk false))))

(fn `UserConstructionScript`)