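; BP_Dendron is the Blueprint for the Dendron enemy, handling its laser visibility and its idle and alert eye states.
; Custom events show or hide the Niagara laser, while Search_Eye and TargetScan_Eye swap idle or alert materials on the scan eye and both wing lights.
; Search_Eye also clears the line trace flag.
; Tick and BeginPlay are empty, and nothing in this graph calls these events.
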(event `self.ReceiveBeginPlay`)

(event `VisibleLaser`
  (`SceneComponent.SetHiddenInGame` (`self.Niagara`) false false))

(event `HiddenLaser`
  (`SceneComponent.SetHiddenInGame` (`self.Niagara`) true false))

(event `self.ReceiveTick`
  (params (DeltaSeconds :type "Float (single-precision)")))

(event `Search_Eye`
  (`PrimitiveComponent.SetMaterial` (`self.ScanEye`) 0 "/Game/Enemy/Dendron/FX/Dendron_Idle.Dendron_Idle")
  (`PrimitiveComponent.SetMaterial` (`self.RightWingLight`) 0 "/Game/Enemy/Dendron/FX/Dendron_Idle.Dendron_Idle")
  (`PrimitiveComponent.SetMaterial` (`self.LeftWingLight`) 0 "/Game/Enemy/Dendron/FX/Dendron_Idle.Dendron_Idle")
  (set `self.bIsLineTraceActive` false))

(event `TargetScan_Eye`
  (`PrimitiveComponent.SetMaterial` (`self.ScanEye`) 0 "/Game/Enemy/Dendron/FX/Dendron_Alert.Dendron_Alert")
  (`PrimitiveComponent.SetMaterial` (`self.RightWingLight`) 0 "/Game/Enemy/Dendron/FX/Dendron_Alert.Dendron_Alert")
  (`PrimitiveComponent.SetMaterial` (`self.LeftWingLight`) 0 "/Game/Enemy/Dendron/FX/Dendron_Alert.Dendron_Alert"))

(fn `UserConstructionScript`)