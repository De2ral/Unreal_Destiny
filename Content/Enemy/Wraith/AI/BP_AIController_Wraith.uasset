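; AI controller for the Wraith enemy that tracks how close its pawn is to an actor stored in the Blackboard.
; Tick passes through a one-second Delay, so the distance checks run about once per second rather than every frame.
; Two range checks, a nearer and a farther one, each write their own Blackboard bool.
; Possess and BeginPlay are empty, so this graph starts no Behavior Tree.
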(event `self.ReceivePossess`
  (params (PossessedPawn :type "Pawn Object Reference")))

(event `self.ReceiveTick`
  (params (DeltaSeconds :type "Float (single-precision)"))
  (bind _returnvalue (`AIBlueprintHelperLibrary.GetBlackboard` null))
  (bind _key_name_2 (`self.Key Name_2`))
  (bind _returnvalue_2 (`BlackboardComponent.GetValueAsObject` _returnvalue (`self.Key Name_0`)))
  (`KismetSystemLibrary.Delay` 1.0)
  (`|ExecutionSequence`
    (:`then_0`
      (bind `_as액터` (cast `Actor` _returnvalue_2))
      (if (< (`KismetMathLibrary.Vector_Distance` (`self.K2_GetActorLocation` (`self.K2_GetPawn`)) (`self.K2_GetActorLocation` `_as액터`)) 2500.0)
        (`BlackboardComponent.SetValueAsBool` _returnvalue (`self.Key Name_1`) true)
        (else
          (`BlackboardComponent.SetValueAsBool` _returnvalue (`self.Key Name_1`) false))))
    (:`then_1`
      (bind `_as액터_2` (cast `Actor` _returnvalue_2))
      (if (< (`KismetMathLibrary.Vector_Distance` (`self.K2_GetActorLocation` (`self.K2_GetPawn`)) (`self.K2_GetActorLocation` `_as액터_2`)) 4000.0)
        (`BlackboardComponent.SetValueAsBool` _returnvalue _key_name_2 true)
        (else
          (`BlackboardComponent.SetValueAsBool` _returnvalue _key_name_2 false))))))

(fn `UserConstructionScript`)