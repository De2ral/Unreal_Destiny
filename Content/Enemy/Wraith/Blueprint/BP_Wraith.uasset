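; BP_Wraith is a Wraith enemy that shows health and damage feedback when shot and ragdolls on death.
; Its health bar widget turns to the camera's yaw each tick, and hits from "Bullets"-tagged actors refresh it from HP.
; Those hits also screen-project the damage widget at the impact, flagging criticals through CriticalHitBox.
; Death events remove both widgets and switch the mesh to physics.
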(event `self.ReceiveTick`
  (params (DeltaSeconds :type "Float (single-precision)"))
  (bind _progressbar_wraith (`self.ProgressBar_Wraith`))
  (bind (_returnvalue_roll _returnvalue_pitch _returnvalue_yaw) (`KismetMathLibrary.BreakRotator` (`PlayerCameraManager.GetCameraRotation` (`GameplayStatics.GetPlayerCameraManager` 0))))
  (`/Engine/EditorBlueprintResources/StandardMacros.IsValid` _progressbar_wraith
    (:`Is Valid`
      (`SceneComponent.K2_SetWorldRotation` _progressbar_wraith (`KismetMathLibrary.MakeRotator` 0.0 0.0 (+ _returnvalue_yaw 180.0)) false false))))

(event `self.ReceiveHit`
  (params (MyComp :type "PrimitiveComponent Object Reference") (Other :type "Actor Object Reference") (OtherComp :type "PrimitiveComponent Object Reference") (bSelfMoved :type Boolean) (HitLocation :type "Vector Structure") (HitNormal :type "Vector Structure") (NormalImpulse :type "Vector Structure") (Hit :type "HitResult Structure (by ref)"))
  (if (`self.ActorHasTag` Other "Bullets")
    (if (not (`self.isDead`))
      (bind _asprogress_bar_wraith_ (cast `/Game/Enemy/Wraith/UI/ProgressBar_Wraith_` (`WidgetComponent.GetWidget` (`self.ProgressBar_Wraith`))))
      (`ProgressBar.SetPercent` (`/Game/Enemy/Wraith/UI/ProgressBar_Wraith_.ProgressBar` _asprogress_bar_wraith_) (/ (`self.HP`) 100.0))
      (bind _asdamage_widget (cast `/Game/Enemy/Dorongo/UI/Damage_Widget` (`WidgetComponent.GetWidget` (`self.Damage_Widget`))))
      (if (`PrimitiveComponent.IsOverlappingActor` (`self.CriticalHitBox`) Other)
        (`/Game/Enemy/Dorongo/UI/Damage_Widget.Apply Damage` _asdamage_widget (`KismetTextLibrary.Conv_DoubleToText` (`self.DamageValue`) "HalfToEven") false)
        (set `/Game/Enemy/Dorongo/UI/Damage_Widget.CriticalText` true _asdamage_widget)
        (else
          (set `/Game/Enemy/Dorongo/UI/Damage_Widget.CriticalText` false _asdamage_widget)))
      (set `Widget.RenderTransform` (make `WidgetTransform` (`GameplayStatics.ProjectWorldToScreen` null HitLocation)) _asdamage_widget))))

(event `Dead_First`
  (bind _damage_widget (`self.Damage_Widget`))
  (bind _progressbar_wraith (`self.ProgressBar_Wraith`))
  (`/Engine/EditorBlueprintResources/StandardMacros.IsValid` _progressbar_wraith
    (:`Is Valid`
      (`ActorComponent.K2_DestroyComponent` _progressbar_wraith)
      (`/Engine/EditorBlueprintResources/StandardMacros.IsValid` _damage_widget
        (:`Is Valid`
          (`ActorComponent.K2_DestroyComponent` _damage_widget))))))

(event `Death_Ragdoll`
  (bind _mesh (`self.Mesh`))
  (`PrimitiveComponent.SetSimulatePhysics` _mesh true)
  (`PrimitiveComponent.SetCollisionProfileName` _mesh "PhysicsActor" true)
  (set `PrimitiveComponent.bGenerateOverlapEvents` false _mesh)
  (`PrimitiveComponent.SetCollisionEnabled` (`self.CapsuleComponent`) "NoCollision"))

(event `self.ReceiveAnyDamage`
  (params (Damage :type "Float (single-precision)") (DamageType :type "DamageType Object Reference") (InstigatedBy :type "Controller Object Reference") (DamageCauser :type "Actor Object Reference"))
  (if (`self.isDead`)
    (set `self.DamageText` Damage)
    (else
      (`self.RandomPosition`)
      (set `self.Progress_HP` (`self.HP`))
      (set `self.DamageText` Damage))))

(event `self.CriticalHitBox.OnComponentHit`
  (params (HitComponent :type "PrimitiveComponent Object Reference") (OtherActor :type "Actor Object Reference") (OtherComp :type "PrimitiveComponent Object Reference") (NormalImpulse :type "Vector Structure") (Hit :type "HitResult Structure (by ref)"))
  (bind _asdamage_widget (cast `/Game/Enemy/Dorongo/UI/Damage_Widget` (`WidgetComponent.GetWidget` (`self.Damage_Widget`))))
  (set `/Game/Enemy/Dorongo/UI/Damage_Widget.CriticalText` true _asdamage_widget))

(fn `LowHP`
  (if (<= (`self.HP`) 20.0)
    (return)))

(fn `OnRep_DamageText`)

(fn `OnRep_Progress_HP`)

(fn `RandomPosition`
  (bind _y (.y (`SceneComponent.K2_GetComponentLocation` (`self.WidgetPoint`))))
  (bind _z (.z (`SceneComponent.K2_GetComponentLocation` (`self.WidgetPoint`))))
  (set `self.RandomDamagePoint` (`KismetMathLibrary.MakeVector` (.x (`SceneComponent.K2_GetComponentLocation` (`self.WidgetPoint`))) (`KismetMathLibrary.RandomFloatInRange` (- _y 100.0) (+ _y 100.0)) (`KismetMathLibrary.RandomFloatInRange` (- _z 100.0) (+ _z 100.0)))))

(fn `UserConstructionScript`)