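; Wraith enemy Blueprint that handles health-bar display, floating damage numbers and death cleanup.
; Tick turns the health-bar widget toward the player camera by yaw only.
; AnyDamage updates the bar from HP after a short delay and spawns a damage-number actor at a randomized offset around WidgetPoint.
; Death events remove the widgets and switch the mesh to ragdoll; an older bullet-hit widget path is disconnected, and LowHP does nothing.
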(event `self.ReceiveTick`
  (params (DeltaSeconds :type "Float (single-precision)"))
  (bind _progressbar_wraith (`self.ProgressBar_Wraith`))
  (bind (_returnvalue_roll _returnvalue_pitch _returnvalue_yaw) (`KismetMathLibrary.BreakRotator` (`PlayerCameraManager.GetCameraRotation` (`GameplayStatics.GetPlayerCameraManager` 0))))
  (`/Engine/EditorBlueprintResources/StandardMacros.IsValid` _progressbar_wraith
    (:`Is Valid`
      (`SceneComponent.K2_SetWorldRotation` _progressbar_wraith (`KismetMathLibrary.MakeRotator` 0.0 0.0 (+ _returnvalue_yaw 180.0)) false false))))

(event `self.ReceiveHit`
  (params (MyComp :type "PrimitiveComponent Object Reference") (Other :type "Actor Object Reference") (OtherComp :type "PrimitiveComponent Object Reference") (bSelfMoved :type Boolean) (HitLocation :type "Vector Structure") (HitNormal :type "Vector Structure") (NormalImpulse :type "Vector Structure") (Hit :type "HitResult Structure (by ref)")))

(event `Dead_First`
  (bind _damage_widget_wraith (`self.Damage_Widget_Wraith`))
  (bind _progressbar_wraith (`self.ProgressBar_Wraith`))
  (`/Engine/EditorBlueprintResources/StandardMacros.IsValid` _progressbar_wraith
    (:`Is Valid`
      (`ActorComponent.K2_DestroyComponent` _progressbar_wraith)
      (`/Engine/EditorBlueprintResources/StandardMacros.IsValid` _damage_widget_wraith
        (:`Is Valid`
          (`ActorComponent.K2_DestroyComponent` _damage_widget_wraith))))))

(event `Death_Ragdoll`
  (bind _mesh (`self.Mesh`))
  (`PrimitiveComponent.SetSimulatePhysics` (`self.Mesh`) true)
  (`PrimitiveComponent.SetCollisionProfileName` _mesh "PhysicsActor" true)
  (set `PrimitiveComponent.bGenerateOverlapEvents` false _mesh)
  (`PrimitiveComponent.SetCollisionEnabled` (`self.CapsuleComponent`) "NoCollision"))

(event `self.ReceiveAnyDamage`
  (params (Damage :type "Float (single-precision)") (DamageType :type "DamageType Object Reference") (InstigatedBy :type "Controller Object Reference") (DamageCauser :type "Actor Object Reference"))
  (`self.RandomPosition`)
  (bind _output_get (set `self.DamageValue` Damage))
  (`KismetSystemLibrary.Delay` 0.05)
  (if (not (`self.isDead`))
    (bind _asprogress_bar_wraith (cast `/Game/Enemy/Wraith/UI/ProgressBar_Wraith` (`WidgetComponent.GetWidget` (`self.ProgressBar_Wraith`))))
    (`ProgressBar.SetPercent` (`/Game/Enemy/Wraith/UI/ProgressBar_Wraith.ProgressBar` _asprogress_bar_wraith) (/ (`self.HP`) 100.0))
    (bind _returnvalue (`|SpawnActorFromClass` "/Game/Enemy/Dorongo/UI/DamageWidget_Actor.DamageWidget_Actor_C" (`KismetMathLibrary.MakeTransform` (`self.RandomDamagePoint`)) "Undefined" "OverrideRootScale" null null))
    (`/Game/Enemy/Dorongo/UI/DamageWidget_Actor.SetDamageValue` _returnvalue _output_get)))

(fn `LowHP`
  (if (<= (`self.HP`) 20.0)
    (return)))

(fn `RandomPosition`
  (bind _y (.y (`SceneComponent.K2_GetComponentLocation` (`self.WidgetPoint`))))
  (bind _z (.z (`SceneComponent.K2_GetComponentLocation` (`self.WidgetPoint`))))
  (set `self.RandomDamagePoint` (`KismetMathLibrary.MakeVector` (.x (`SceneComponent.K2_GetComponentLocation` (`self.WidgetPoint`))) (`KismetMathLibrary.RandomFloatInRange` (- _y 100.0) (+ _y 100.0)) (`KismetMathLibrary.RandomFloatInRange` (- _z 100.0) (+ _z 100.0)))))

(fn `UserConstructionScript`)