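; BP_Exploder is an enemy character that shows a health bar and damage numbers when hit.
; Tick turns the widget to face the camera's yaw.
; AnyDamage waits briefly, then either updates the bar and spawns a damage-number actor at a random offset, or, if IsDead, removes widgets and collision.
; Attack only casts the AI controller; the range overlap is empty and the delayed player-damage logic is unconnected.
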(event `self.ReceiveTick`
  (params (DeltaSeconds :type "Float (single-precision)"))
  (bind _widget (`self.Widget`))
  (bind (_returnvalue_roll _returnvalue_pitch _returnvalue_yaw) (`KismetMathLibrary.BreakRotator` (`PlayerCameraManager.GetCameraRotation` (`GameplayStatics.GetPlayerCameraManager` 0))))
  (`/Engine/EditorBlueprintResources/StandardMacros.IsValid` _widget
    (:`Is Valid`
      (`SceneComponent.K2_SetWorldRotation` _widget (`KismetMathLibrary.MakeRotator` 0.0 0.0 (+ _returnvalue_yaw 180.0)) false false))))

(event `self.ReceiveAnyDamage`
  (params (Damage :type "Float (single-precision)") (DamageType :type "DamageType Object Reference") (InstigatedBy :type "Controller Object Reference") (DamageCauser :type "Actor Object Reference"))
  (bind _widget (`self.Widget`))
  (bind _damage_widget (`self.Damage_Widget`))
  (bind _mesh (`self.Mesh`))
  (`self.RandomPosition`)
  (bind _output_get (set `self.DamageValue` Damage))
  (`KismetSystemLibrary.Delay` 0.05)
  (if (`self.isDead`)
    (`/Engine/EditorBlueprintResources/StandardMacros.IsValid` _widget
      (:`Is Valid`
        (`ActorComponent.K2_DestroyComponent` _widget)
        (`/Engine/EditorBlueprintResources/StandardMacros.IsValid` _damage_widget
          (:`Is Valid`
            (`ActorComponent.K2_DestroyComponent` _damage_widget)
            (`PrimitiveComponent.SetCollisionProfileName` _mesh "None" true)
            (set `PrimitiveComponent.bGenerateOverlapEvents` false _mesh)
            (`PrimitiveComponent.SetCollisionEnabled` (`self.CapsuleComponent`) "NoCollision")))))
    (else
      (bind _asprogress_bar_exploder (cast `/Game/Enemy/Exploder/UI/ProgressBar_Exploder` (`WidgetComponent.GetWidget` (`self.Widget`))))
      (`ProgressBar.SetPercent` (`/Game/Enemy/Exploder/UI/ProgressBar_Exploder.ProgressBar` _asprogress_bar_exploder) (/ (`self.HP`) 100.0))
      (bind _returnvalue (`|SpawnActorFromClass` "/Game/Enemy/Dorongo/UI/DamageWidget_Actor.DamageWidget_Actor_C" (`KismetMathLibrary.MakeTransform` (`self.RandomDamagePoint`)) "Undefined" "OverrideRootScale" null null))
      (`/Game/Enemy/Dorongo/UI/DamageWidget_Actor.SetDamageValue` _returnvalue _output_get))))

(event `self.Sphere_Range.OnComponentBeginOverlap`
  (params (OverlappedComponent :type "PrimitiveComponent Object Reference") (OtherActor :type "Actor Object Reference") (OtherComp :type "PrimitiveComponent Object Reference") (OtherBodyIndex :type Integer) (bFromSweep :type Boolean) (SweepResult :type "HitResult Structure (by ref)")))

(event `Attack`
  (cast `/Game/Enemy/Exploder/AI/AIC_Exploder` (`AIBlueprintHelperLibrary.GetAIController` self)))

(fn `RandomPosition`
  (bind _y (.y (`SceneComponent.K2_GetComponentLocation` (`self.WidgetPoint`))))
  (bind _z (.z (`SceneComponent.K2_GetComponentLocation` (`self.WidgetPoint`))))
  (set `self.RandomDamagePoint` (`KismetMathLibrary.MakeVector` (.x (`SceneComponent.K2_GetComponentLocation` (`self.WidgetPoint`))) (`KismetMathLibrary.RandomFloatInRange` (- _y 100.0) (+ _y 100.0)) (`KismetMathLibrary.RandomFloatInRange` (- _z 100.0) (+ _z 100.0)))))

(fn `UserConstructionScript`)