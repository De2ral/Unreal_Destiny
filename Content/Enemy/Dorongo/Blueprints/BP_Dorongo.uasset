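; Dorongo enemy character that reacts to bullets and damage with a health bar, damage numbers and a random dodge, plus ragdoll and UI cleanup events for death.
; The health bar yaws toward the camera each tick, while bullet hits update it and flag criticals through CriticalHitBox overlap.
; AnyDamage sets ProgressHP and DamageText, whose OnRep functions refresh the bar and spawn damage-number actors.
; The Turn macro occasionally faces the player and launches sideways.
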(event `self.ReceiveTick`
  (params (DeltaSeconds :type "Float (single-precision)"))
  (bind _widget (`self.Widget`))
  (bind (_returnvalue_roll _returnvalue_pitch _returnvalue_yaw) (`KismetMathLibrary.BreakRotator` (`PlayerCameraManager.GetCameraRotation` (`GameplayStatics.GetPlayerCameraManager` 0))))
  (`/Engine/EditorBlueprintResources/StandardMacros.IsValid` _widget
    (:`Is Valid`
      (`SceneComponent.K2_SetWorldRotation` _widget (`KismetMathLibrary.MakeRotator` 0.0 0.0 (+ _returnvalue_yaw 180.0)) false false))))

(event `self.ReceiveHit`
  (params (MyComp :type "PrimitiveComponent Object Reference") (Other :type "Actor Object Reference") (OtherComp :type "PrimitiveComponent Object Reference") (bSelfMoved :type Boolean) (HitLocation :type "Vector Structure") (HitNormal :type "Vector Structure") (NormalImpulse :type "Vector Structure") (Hit :type "HitResult Structure (by ref)"))
  (if (`self.ActorHasTag` Other "Bullets")
    (`self.Turn`
      (:`then`
        _)
      (:`then2`
        _))
    (if (not (`self.isDead`))
      (bind _asprogress_bar_dorongo (cast `/Game/Enemy/Dorongo/UI/ProgressBar_Dorongo` (`WidgetComponent.GetWidget` (`self.Widget`))))
      (`ProgressBar.SetPercent` (`/Game/Enemy/Dorongo/UI/ProgressBar_Dorongo.ProgressBar` _asprogress_bar_dorongo) (/ (`self.HP`) 100.0))
      (bind _asdamage_widget (cast `/Game/Enemy/Dorongo/UI/Damage_Widget` (`WidgetComponent.GetWidget` (`self.Damage_Widget`))))
      (if (`PrimitiveComponent.IsOverlappingActor` (`self.CriticalHitBox`) Other)
        (`/Game/Enemy/Dorongo/UI/Damage_Widget.Apply Damage` _asdamage_widget (`KismetTextLibrary.Conv_DoubleToText` (`self.DamageValue`) "HalfToEven") false)
        (set `/Game/Enemy/Dorongo/UI/Damage_Widget.CriticalText` true _asdamage_widget)
        (else
          (set `/Game/Enemy/Dorongo/UI/Damage_Widget.CriticalText` false _asdamage_widget)))
      (set `Widget.RenderTransform` (make `WidgetTransform` (`GameplayStatics.ProjectWorldToScreen` null HitLocation)) _asdamage_widget))))

(event `Death_Ragdoll`
  (bind _mesh (`self.Mesh`))
  (`PrimitiveComponent.SetSimulatePhysics` (`self.Mesh`) true)
  (`PrimitiveComponent.SetCollisionProfileName` _mesh "PhysicsActor" true)
  (set `PrimitiveComponent.bGenerateOverlapEvents` false _mesh)
  (`PrimitiveComponent.SetCollisionEnabled` (`self.CapsuleComponent`) "NoCollision"))

(event `Dead_First`
  (bind _damage_widget (`self.Damage_Widget`))
  (bind _widget (`self.Widget`))
  (`/Engine/EditorBlueprintResources/StandardMacros.IsValid` _widget
    (:`Is Valid`
      (`ActorComponent.K2_DestroyComponent` _widget)
      (`/Engine/EditorBlueprintResources/StandardMacros.IsValid` _damage_widget
        (:`Is Valid`
          (`ActorComponent.K2_DestroyComponent` _damage_widget))))))

(event `Attacking`)

(event `self.ReceiveAnyDamage`
  (params (Damage :type "Float (single-precision)") (DamageType :type "DamageType Object Reference") (InstigatedBy :type "Controller Object Reference") (DamageCauser :type "Actor Object Reference"))
  (if (`self.isDead`)
    (set `self.DamageText` Damage)
    (else
      (`self.RandomPosition`)
      (set `self.Progress_HP` (`self.HP`))
      (`self.Turn`
        (:`then`
          _)
        (:`then2`
          _))
      (set `self.DamageText` Damage))))

(event `multicast`)

(event `self.CriticalHitBox.OnComponentHit`
  (params (HitComponent :type "PrimitiveComponent Object Reference") (OtherActor :type "Actor Object Reference") (OtherComp :type "PrimitiveComponent Object Reference") (NormalImpulse :type "Vector Structure") (Hit :type "HitResult Structure (by ref)"))
  (bind _asdamage_widget (cast `/Game/Enemy/Dorongo/UI/Damage_Widget` (`WidgetComponent.GetWidget` (`self.Damage_Widget`))))
  (bind _output_get (set `/Game/Enemy/Dorongo/UI/Damage_Widget.CriticalText` true _asdamage_widget))
  (`KismetSystemLibrary.PrintString` (`KismetStringLibrary.Conv_BoolToString` _output_get)))

(event `self.CriticalHitBox.OnComponentBeginOverlap`
  (params (OverlappedComponent :type "PrimitiveComponent Object Reference") (OtherActor :type "Actor Object Reference") (OtherComp :type "PrimitiveComponent Object Reference") (OtherBodyIndex :type Integer) (bFromSweep :type Boolean) (SweepResult :type "HitResult Structure (by ref)")))

(fn `OnRep_DamageText`
  (bind _damagetext (`self.DamageText`))
  (bind _returnvalue (`|SpawnActorFromClass` "/Game/Enemy/Dorongo/UI/DamageWidget_Actor.DamageWidget_Actor_C" (`KismetMathLibrary.MakeTransform` (`self.RandomDamagePoint`)) "Undefined" "OverrideRootScale" null null))
  (if (`self.bIsCriticalTextColor`)
    (`/Game/Enemy/Dorongo/UI/DamageWidget_Actor.SetDamageCriticalValue` _returnvalue (* _damagetext 2.0))
    (else
      (`/Game/Enemy/Dorongo/UI/DamageWidget_Actor.SetDamageValue` _returnvalue _damagetext)))
  (set `self.bIsCriticalTextColor` false))

(fn `OnRep_Progress_HP`
  (bind _asprogress_bar_dorongo (cast `/Game/Enemy/Dorongo/UI/ProgressBar_Dorongo` (`WidgetComponent.GetWidget` (`self.Widget`))))
  (bind _progressbar (`/Game/Enemy/Dorongo/UI/ProgressBar_Dorongo.ProgressBar` _asprogress_bar_dorongo)
    (:`then`
      (`ProgressBar.SetPercent` _progressbar (/ (`self.HP`) 100.0)))
    (:`else`)))

(fn `RandomPosition`
  (bind _y (.y (`SceneComponent.K2_GetComponentLocation` (`self.WidgetPoint`))))
  (bind _z (.z (`SceneComponent.K2_GetComponentLocation` (`self.WidgetPoint`))))
  (set `self.RandomDamagePoint` (`KismetMathLibrary.MakeVector` (.x (`SceneComponent.K2_GetComponentLocation` (`self.WidgetPoint`))) (`KismetMathLibrary.RandomFloatInRange` (- _y 100.0) (+ _y 100.0)) (`KismetMathLibrary.RandomFloatInRange` (- _z 100.0) (+ _z 100.0)))))

(fn `UserConstructionScript`)