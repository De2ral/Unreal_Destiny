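; BP_Galhak is an enemy with a flame attack, twin mine drops and an explosive death.
; Flame events toggle a capsule's collision to damage overlapping players, while mines spawn near sockets.
; AnyDamage feeds RepNotify variables that update the health bar and spawn randomly placed damage numbers, doubled for criticals.
; Bullet hits also update widgets, flagging criticals via CriticalHitBox overlap, and Tick yaws the health bar toward the camera.
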(event `self.ReceiveBeginPlay`
  (`PrimitiveComponent.SetCollisionEnabled` (`self.Capsule`) "NoCollision"))

(event `self.ReceiveTick`
  (params (DeltaSeconds :type "Float (single-precision)"))
  (bind _widget (`self.Widget`))
  (bind (_returnvalue_roll _returnvalue_pitch _returnvalue_yaw) (`KismetMathLibrary.BreakRotator` (`PlayerCameraManager.GetCameraRotation` (`GameplayStatics.GetPlayerCameraManager` 0))))
  (`/Engine/EditorBlueprintResources/StandardMacros.IsValid` _widget
    (:`Is Valid`
      (`SceneComponent.K2_SetWorldRotation` _widget (`KismetMathLibrary.MakeRotator` 0.0 0.0 (+ _returnvalue_yaw 180.0)) false false))))

(event `self.ReceiveAnyDamage`
  (params (Damage :type "Float (single-precision)") (DamageType :type "DamageType Object Reference") (InstigatedBy :type "Controller Object Reference") (DamageCauser :type "Actor Object Reference"))
  (if (`self.isDead`)
    (set `self.DamageText` Damage)
    (else
      (`self.RandomPosition`)
      (set `self.Progress_HP` (`self.HP`))
      (set `self.DamageText` Damage))))

(event `self.ReceiveHit`
  (params (MyComp :type "PrimitiveComponent Object Reference") (Other :type "Actor Object Reference") (OtherComp :type "PrimitiveComponent Object Reference") (bSelfMoved :type Boolean) (HitLocation :type "Vector Structure") (HitNormal :type "Vector Structure") (NormalImpulse :type "Vector Structure") (Hit :type "HitResult Structure (by ref)"))
  (if (`self.ActorHasTag` Other "Bullets")
    (if (not (`self.isDead`))
      (bind _asprogress_bar_galhak (cast `/Game/Enemy/Gahlak/UI/ProgressBar_Galhak` (`WidgetComponent.GetWidget` (`self.Widget`))))
      (`ProgressBar.SetPercent` (`/Game/Enemy/Gahlak/UI/ProgressBar_Galhak.ProgressBar` _asprogress_bar_galhak) (/ (`self.HP`) 100.0))
      (bind _asdamage_widget_galhak (cast `/Game/Enemy/Gahlak/UI/Damage_Widget_Galhak` (`WidgetComponent.GetWidget` (`self.Damage Widget`))))
      (if (`PrimitiveComponent.IsOverlappingActor` (`self.CriticalHitBox`) Other)
        (`/Game/Enemy/Gahlak/UI/Damage_Widget_Galhak.Apply Damage` _asdamage_widget_galhak (`KismetTextLibrary.Conv_DoubleToText` (`self.DamageValue`) "HalfToEven") false)
        (set `/Game/Enemy/Gahlak/UI/Damage_Widget_Galhak.CriticalText` true _asdamage_widget_galhak)
        (else
          (set `/Game/Enemy/Gahlak/UI/Damage_Widget_Galhak.CriticalText` false _asdamage_widget_galhak)))
      (set `Widget.RenderTransform` (make `WidgetTransform` (`GameplayStatics.ProjectWorldToScreen` null HitLocation)) _asdamage_widget_galhak))))

(event `Dead_First`
  (bind _widget (`self.Widget`))
  (bind _damage_widget (`self.Damage Widget`))
  (`/Engine/EditorBlueprintResources/StandardMacros.IsValid` _widget
    (:`Is Valid`
      (`ActorComponent.K2_DestroyComponent` _widget)
      (`/Engine/EditorBlueprintResources/StandardMacros.IsValid` _damage_widget
        (:`Is Valid`
          (`ActorComponent.K2_DestroyComponent` _damage_widget))))))

(event `Death_Ragdoll`
  (bind _mesh (`self.Mesh`))
  (`PrimitiveComponent.SetCollisionProfileName` _mesh "PhysicsActor" true)
  (set `PrimitiveComponent.bGenerateOverlapEvents` false _mesh)
  (`PrimitiveComponent.SetCollisionEnabled` (`self.CapsuleComponent`) "NoCollision")
  (`KismetSystemLibrary.Delay` 0.1)
  (`GameplayStatics.SpawnEmitterAtLocation` "/Game/Enemy/Exploder/FX/expbomb.expbomb" (`self.K2_GetActorLocation`) (struct))
  (`ActorComponent.K2_DestroyComponent` (`self.Mesh`))
  (`ActorComponent.K2_DestroyComponent` (`self.Weapon`))
  (`self.K2_DestroyActor`))

(event `self.Capsule.OnComponentBeginOverlap`
  (params (OverlappedComponent :type "PrimitiveComponent Object Reference") (OtherActor :type "Actor Object Reference") (OtherComp :type "PrimitiveComponent Object Reference") (OtherBodyIndex :type Integer) (bFromSweep :type Boolean) (SweepResult :type "HitResult Structure (by ref)"))
  (if (`self.ActorHasTag` OtherActor "DestinyPlayer")
    (`GameplayStatics.ApplyDamage` OtherActor 5.0)))

(event `Death_Effect_OnServer`
  (`self.Death_Effect_Multicast`))

(event `Death_Effect_Multicast`
  (`GameplayStatics.SpawnEmitterAtLocation` "/Game/Enemy/Exploder/FX/expbomb.expbomb"))

(event `FlameAttackStart`
  (`PrimitiveComponent.SetCollisionEnabled` (`self.Capsule`) "QueryAndPhysics"))

(event `FlameAttackEnd`
  (`PrimitiveComponent.SetCollisionEnabled` (`self.Capsule`) "NoCollision"))

(event `Fire Mine Start`
  (bind (_returnvalue_x _returnvalue_y _returnvalue_z) (`KismetMathLibrary.BreakVector` (`SceneComponent.GetSocketLocation` (`self.L_Mine`) "R_Mine_Socket")))
  (bind (_returnvalue_x_2 _returnvalue_y_2 _returnvalue_z_2) (`KismetMathLibrary.BreakVector` (`SceneComponent.GetSocketLocation` (`self.R_Mine`) "L_Miine_Socket")))
  (`|ExecutionSequence`
    (:`then_0`
      (`|SpawnActorFromClass` "/Game/Enemy/Gahlak/Bluprint/BP_Mine_Galhaks.BP_Mine_Galhaks_C" (`KismetMathLibrary.MakeTransform` (`KismetMathLibrary.MakeVector` _returnvalue_x_2 (+ _returnvalue_y_2 30.0) _returnvalue_z_2)) "Undefined" "OverrideRootScale" null null)
      (`KismetSystemLibrary.PrintString` "L _ Mine"))
    (:`then_1`
      (`|SpawnActorFromClass` "/Game/Enemy/Gahlak/Bluprint/BP_Mine_Galhaks.BP_Mine_Galhaks_C" (`KismetMathLibrary.MakeTransform` (`KismetMathLibrary.MakeVector` _returnvalue_x (+ _returnvalue_y 50.0) _returnvalue_z)) "Undefined" "OverrideRootScale" null null)
      (`KismetSystemLibrary.PrintString` "R _ Mine"))))

(fn `OnRep_DamageText`
  (bind _damagetext (`self.DamageText`))
  (bind _returnvalue (`|SpawnActorFromClass` "/Game/Enemy/Dorongo/UI/DamageWidget_Actor.DamageWidget_Actor_C" (`KismetMathLibrary.MakeTransform` (`self.RandomDamagePoint`)) "Undefined" "OverrideRootScale" null null))
  (if (`self.bIsCriticalTextColor`)
    (`/Game/Enemy/Dorongo/UI/DamageWidget_Actor.SetDamageCriticalValue` _returnvalue (* _damagetext 2.0))
    (else
      (`/Game/Enemy/Dorongo/UI/DamageWidget_Actor.SetDamageValue` _returnvalue _damagetext)))
  (set `self.bIsCriticalTextColor` false))

(fn `OnRep_Progress_HP`
  (bind _asprogress_bar_galhak (cast `/Game/Enemy/Gahlak/UI/ProgressBar_Galhak` (`WidgetComponent.GetWidget` (`self.Widget`))))
  (bind _progressbar (`/Game/Enemy/Gahlak/UI/ProgressBar_Galhak.ProgressBar` _asprogress_bar_galhak)
    (:`then`
      (`ProgressBar.SetPercent` _progressbar (/ (`self.HP`) 100.0)))
    (:`else`)))

(fn `RandomPosition`
  (bind _y (.y (`SceneComponent.K2_GetComponentLocation` (`self.WidgetPoint`))))
  (bind _z (.z (`SceneComponent.K2_GetComponentLocation` (`self.WidgetPoint`))))
  (set `self.RandomDamagePoint` (`KismetMathLibrary.MakeVector` (.x (`SceneComponent.K2_GetComponentLocation` (`self.WidgetPoint`))) (`KismetMathLibrary.RandomFloatInRange` (- _y 100.0) (+ _y 100.0)) (`KismetMathLibrary.RandomFloatInRange` (- _z 100.0) (+ _z 100.0)))))

(fn `UserConstructionScript`)

(fn `새 함수`)