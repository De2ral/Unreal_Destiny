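; Heal aura actor for the Heraklios Mage enemy that adds a fixed amount to the mage's HP.
; Server events forward to client counterparts, which spawn a flattened particle aura, size the sphere, and remove the effect after Duration.
; The heal event sets interval and duration timers, applies the HP gain and calls DestroyActor.
; SpawnSphere scans for nearby pawns and notifies each, but only when the DrawDebugSphere flag is on.
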(event `self.Sphere.OnComponentBeginOverlap`
  (params (OverlappedComponent :type "PrimitiveComponent Object Reference") (OtherActor :type "Actor Object Reference") (OtherComp :type "PrimitiveComponent Object Reference") (OtherBodyIndex :type Integer) (bFromSweep :type Boolean) (SweepResult :type "HitResult Structure (by ref)")))

(event `HealAura_ On Client`
  (bind _as_bp_mage (`self.As BP Mage`))
  (`self.SpawnEffect_client`)
  (`|ExecutionSequence`
    (:`then_0`
      (`KismetSystemLibrary.K2_SetTimerDelegate` (`|CreateDelegate` :!event `HealAura_On Server`) (`self.SpawnInterval`))
      (set `CPP_MonsterBase.HP` (+ (`CPP_MonsterBase.HP` _as_bp_mage) 30.0) _as_bp_mage)
      (`KismetSystemLibrary.PrintString` "Mage_Heal"))
    (:`then_1`
      (`KismetSystemLibrary.K2_SetTimerDelegate` (`|CreateDelegate` :!event `K2_DestroyActor`) (`self.Duration`))
      (`self.K2_DestroyActor`))))

(event `HealAura_On Server`
  (`self.HealAura_ On Client`))

(event `SpawnSphere`
  (if (`self.DrawDebugSphere`)
    (`KismetSystemLibrary.DrawDebugSphere` (`self.K2_GetActorLocation`) (`self.Sphere Radius`) 12 (struct :`R` 1.0 :`B` 0.723844 :`A` 1.0) 2.0 1.0)
    (bind _outactors (`KismetSystemLibrary.SphereOverlapActors` (`self.K2_GetActorLocation`) (`self.Sphere Radius`) (`|MakeArray` "ObjectTypeQuery3" :!type "EObjectTypeQuery Enum") null (select `bool` (`self.IgnoreInstigator`) :`true` (`|MakeArray` (`self.GetInstigator`) :!type "Actor Object Reference"))))
    (for _array_element _outactors
      (`self.OnAuraOverlapActor` _array_element))))

(event `SpawnEffect_client`
  (bind (_returnvalue_x _returnvalue_y _returnvalue_z) (`KismetMathLibrary.BreakVector` (`self.K2_GetActorLocation`)))
  (bind _returnvalue (`GameplayStatics.SpawnEmitterAtLocation` "/Game/Particle_Packs/Heal/Particles/P_ky_healAura.P_ky_healAura" (`KismetMathLibrary.MakeVector` _returnvalue_x _returnvalue_y (- _returnvalue_z 80.0)) (struct) (3.0 3.0 0.1)))
  (`SphereComponent.SetSphereRadius` (`self.Sphere`) (`self.Sphere Radius`) true)
  (`KismetSystemLibrary.Delay` (`self.Duration`))
  (`ActorComponent.K2_DestroyComponent` _returnvalue))

(event `SpawnEffect_Server`
  (`self.SpawnEffect_client`))

(fn `UserConstructionScript`)