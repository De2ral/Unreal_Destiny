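; Consecrated Mind boss: a slowly rotating enemy with red, green and blue core states, mirrored to its AI blackboard.
; RepNotify variables drive the boss HUD health bar and floating damage numbers.
; Below half health it flags a one-time super-power phase (state 3), with separate events for white core, shield and Boss_Field orbs.
; A WhitePatternCount of three ends that phase, destroying the shield and rerolling a non-repeating color.
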(event `self.ReceiveAnyDamage`
  (params (Damage :type "Float (single-precision)") (DamageType :type "DamageType Object Reference") (InstigatedBy :type "Controller Object Reference") (DamageCauser :type "Actor Object Reference"))
  (bind _returnvalue (`AIBlueprintHelperLibrary.GetBlackboard` null))
  (`|ExecutionSequence`
    (:`then_0`
      (if (`self.isDead`)
        (set `self.DamageText` Damage)
        (else
          (`self.RandomPosition`)
          (set `self.Progress_HP` (`self.HP`))
          (set `self.DamageText` Damage))))
    (:`then_1`
      (if (< (`self.HP`) 10000.0)
        (`/Engine/EditorBlueprintResources/StandardMacros.DoOnce` false
          (:`Completed`
            (if (`KismetSystemLibrary.IsValid` _returnvalue)
              (`BlackboardComponent.SetValueAsInt` _returnvalue (`self.Key_StateNum`) 3)
              (`BlackboardComponent.SetValueAsBool` _returnvalue (`self.Key Name`) true)
              (set `self.isSuperPower` true))))))))

(event `self.ReceiveBeginPlay`
  (set `self.HP` 20000.0)
  (bind _returnvalue (`|CreateWidget` "/Game/Enemy/Boss_ConsecratedMind/UI/Boss_HUD.Boss_HUD_C"))
  (bind _output_get (set `self.HUD` _returnvalue))
  (`UserWidget.AddToViewport` _returnvalue 0)
  (`Widget.SetVisibility` (`/Game/Enemy/Boss_ConsecratedMind/UI/Boss_HUD.Boss_Canvas` _output_get) "Hidden"))

(event `UI_Visible`
  (`Widget.SetVisibility` (`/Game/Enemy/Boss_ConsecratedMind/UI/Boss_HUD.Boss_Canvas` (stale `self.ReceiveBeginPlay` _output_get)) "Visible"))

(event `SpawnOrb`
  (bind _returnvalue (`GameplayStatics.GetActorOfClass` "/Game/Enemy/Boss_ConsecratedMind/Blueprints/Boss_Field.Boss_Field_C"))
  (`/Game/Enemy/Boss_ConsecratedMind/Blueprints/Boss_Field.Spawn Orb` _returnvalue)
  (`SceneComponent.SetHiddenInGame` (`self.Shield`) false false))

(event `self.ReceiveTick`
  (params (DeltaSeconds :type "Float (single-precision)"))
  (`SceneComponent.K2_AddWorldRotation` (`self.CapsuleComponent`) (struct :`Yaw` 0.2) false false))

(event `StateChange`
  (bind _output_get (set `self.StateNum` (`KismetMathLibrary.RandomIntegerInRange` (`self.StateNum`) 2)))
  (if (== (`self.StateNum`) (`self.PreStateNum`)) :!label _label
    (set `self.StateNum` (`KismetMathLibrary.RandomIntegerInRange` 0 2))
    (goto _label)
    (else
      (set `self.PreStateNum` _output_get)
      (switch `int` _output_get
        (:`0`
          (`self.StateRed`))
        (:`1`
          (`self.StateGreen`))
        (:`2`
          (`self.StateBlue`))))))

(event `StateWhite`
  (`self.StateWhite_Multicast`))

(event `StateWhite_Multicast`
  (bind _returnvalue (`AIBlueprintHelperLibrary.GetBlackboard` null))
  (`PrimitiveComponent.SetMaterial` (`self.CoreMesh`) 0 "/Game/Enemy/Boss_ConsecratedMind/FX/Core_White.Core_White")
  (if (`KismetSystemLibrary.IsValid` _returnvalue)
    (`BlackboardComponent.SetValueAsInt` _returnvalue (`self.Key_StateNum`) 3)))

(event `StateRed`
  (bind _returnvalue (`AIBlueprintHelperLibrary.GetBlackboard` null))
  (`PrimitiveComponent.SetMaterial` (`self.CoreMesh`) 0 "/Game/Enemy/Boss_ConsecratedMind/FX/Core_Red.Core_Red")
  (if (`KismetSystemLibrary.IsValid` _returnvalue) :!label _label_2
    (`BlackboardComponent.SetValueAsInt` _returnvalue (`self.Key_StateNum`) (`self.StateNum`))))

(event `StateGreen`
  (`PrimitiveComponent.SetMaterial` (`self.CoreMesh`) 0 "/Game/Enemy/Boss_ConsecratedMind/FX/Core_Green.Core_Green")
  (goto _label_2))

(event `StateBlue`
  (`PrimitiveComponent.SetMaterial` (`self.CoreMesh`) 0 "/Game/Enemy/Boss_ConsecratedMind/FX/Core_Blue.Core_Blue")
  (goto _label_2))

(fn `OnRep_DamageText`
  (bind _damagetext (`self.DamageText`))
  (bind _returnvalue (`|SpawnActorFromClass` "/Game/Enemy/Dorongo/UI/DamageWidget_Actor.DamageWidget_Actor_C" (`KismetMathLibrary.MakeTransform` (`self.RandomDamagePoint`)) "Undefined" "OverrideRootScale" null null))
  (if (`self.bIsCriticalTextColor`)
    (`/Game/Enemy/Dorongo/UI/DamageWidget_Actor.SetDamageCriticalValue` _returnvalue (* _damagetext 2.0))
    (else
      (`/Game/Enemy/Dorongo/UI/DamageWidget_Actor.SetDamageValue` _returnvalue _damagetext)))
  (set `self.bIsCriticalTextColor` false))

(fn `OnRep_Progress_HP`
  (bind _hud (`self.HUD`))
  (`/Game/Enemy/Boss_ConsecratedMind/UI/Boss_HUD.HP_Bar_Server` _hud (`self.HP`))
  (bind _boss_bar (`/Game/Enemy/Boss_ConsecratedMind/UI/Boss_HUD.Boss_bar` _hud)
    (:`then`
      (`ProgressBar.SetPercent` _boss_bar (/ (`self.HP`) 20000.0)))
    (:`else`)))

(fn `OnRep_WhitePatternCount`
  (bind _returnvalue (`AIBlueprintHelperLibrary.GetBlackboard` null))
  (bind _shield (`self.Shield`))
  (if (>= (`self.WhitePatternCount`) 3)
    (`self.StateChange`)
    (set `self.isSuperPower` false)
    (if (`KismetSystemLibrary.IsValid` _returnvalue)
      (`BlackboardComponent.SetValueAsBool` _returnvalue (`self.Key Name`) true)
      (`SceneComponent.SetHiddenInGame` _shield true false)
      (`ActorComponent.K2_DestroyComponent` _shield))))

(fn `RandomPosition`
  (bind _y (.y (`SceneComponent.K2_GetComponentLocation` (`self.WidgetPoint`))))
  (bind _z (.z (`SceneComponent.K2_GetComponentLocation` (`self.WidgetPoint`))))
  (set `self.RandomDamagePoint` (`KismetMathLibrary.MakeVector` (.x (`SceneComponent.K2_GetComponentLocation` (`self.WidgetPoint`))) (`KismetMathLibrary.RandomFloatInRange` (- _y 100.0) (+ _y 100.0)) (`KismetMathLibrary.RandomFloatInRange` (- _z 100.0) (+ _z 100.0)))))

(fn `UserConstructionScript`)