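; Boss missile for the Consecrated Mind boss that launches along its mesh's up vector and marks its landing spot with a warning circle.
; On BeginPlay it spawns an Alert_Circle above a calculated impact point and sets a timed self-destruct as a fallback.
; It rotates every tick.
; When its mesh stops overlapping an AlertCircle-tagged component, it destroys that component and itself.
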(event `self.ReceiveBeginPlay`
  (bind (_returnvalue_x _returnvalue_y _returnvalue_z) (`KismetMathLibrary.BreakVector` (`self.CalculateImpactPoint` 1300.0)))
  (`self.LaunchProjectile` (`SceneComponent.GetUpVector` (`self.MeshComponent`)) 4000.0)
  (`|SpawnActorFromClass` "/Game/Enemy/Boss_ConsecratedMind/Blueprints/Alert_Circle.Alert_Circle_C" (`KismetMathLibrary.MakeTransform` (`KismetMathLibrary.MakeVector` _returnvalue_x _returnvalue_y (+ _returnvalue_z 1600.0))) "Undefined" "OverrideRootScale" null null)
  (`KismetSystemLibrary.Delay` 20.0)
  (`self.K2_DestroyActor`))

(event `self.ReceiveTick`
  (params (DeltaSeconds :type "Float (single-precision)"))
  (`self.K2_AddActorWorldRotation` (struct :`Pitch` 2.0)))

(event `self.MeshComponent.OnComponentEndOverlap`
  (params (OverlappedComponent :type "PrimitiveComponent Object Reference") (OtherActor :type "Actor Object Reference") (OtherComp :type "PrimitiveComponent Object Reference") (OtherBodyIndex :type Integer))
  (if (`ActorComponent.ComponentHasTag` OtherComp "AlertCircle")
    (`ActorComponent.K2_DestroyComponent` OtherComp)
    (`self.K2_DestroyActor`)))

(fn `UserConstructionScript`)