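; Field actor for the Consecrated Mind boss that displays rotating attack alerts and reveals orbs.
; SetAlert runs a timeline that shows eight cubes and advances a CustomTime material parameter on eight planes.
; At the time threshold it hides the cubes and rotates Center 25 degrees, repeating once before stopping.
; SpawnOrb unhides three pre-placed orbs and Roll_Reset restores Center's rotation, while ClearAlert is empty.
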(event `self.ReceiveBeginPlay`)

(event `SetAlert`
  (set `self.AlertCount` 1)
  (`Timeline|타임라인` :!via `PlayFromStart` :!label _label
    (:`Update`
      (`SceneComponent.SetHiddenInGame` (`self.Cube2`) false false)
      (`SceneComponent.SetHiddenInGame` (`self.Cube3`) false false)
      (`SceneComponent.SetHiddenInGame` (`self.Cube4`) false false)
      (`SceneComponent.SetHiddenInGame` (`self.Cube5`) false false)
      (`SceneComponent.SetHiddenInGame` (`self.Cube`) false false)
      (`SceneComponent.SetHiddenInGame` (`self.Cube6`) false false)
      (`SceneComponent.SetHiddenInGame` (`self.Cube7`) false false)
      (`SceneComponent.SetHiddenInGame` (`self.Cube1`) false false)
      (bind _output_get (set `self.AlertTime` (+ (`self.AlertTime`) 0.01)))
      (`MeshComponent.SetScalarParameterValueOnMaterials` (`self.Plane`) "CustomTime" _output_get)
      (`MeshComponent.SetScalarParameterValueOnMaterials` (`self.Plane1`) "CustomTime" _output_get)
      (`MeshComponent.SetScalarParameterValueOnMaterials` (`self.Plane7`) "CustomTime" _output_get)
      (`MeshComponent.SetScalarParameterValueOnMaterials` (`self.Plane2`) "CustomTime" _output_get)
      (`MeshComponent.SetScalarParameterValueOnMaterials` (`self.Plane3`) "CustomTime" _output_get)
      (`MeshComponent.SetScalarParameterValueOnMaterials` (`self.Plane6`) "CustomTime" _output_get)
      (`MeshComponent.SetScalarParameterValueOnMaterials` (`self.Plane4`) "CustomTime" _output_get)
      (`MeshComponent.SetScalarParameterValueOnMaterials` (`self.Plane5`) "CustomTime" _output_get)
      (if (> (`self.AlertTime`) 13.0)
        (bind _output_get_2 (set `self.AlertTime` 5.0))
        (`MeshComponent.SetScalarParameterValueOnMaterials` (`self.Plane`) "CustomTime" _output_get_2)
        (`MeshComponent.SetScalarParameterValueOnMaterials` (`self.Plane1`) "CustomTime" _output_get_2)
        (`MeshComponent.SetScalarParameterValueOnMaterials` (`self.Plane7`) "CustomTime" _output_get_2)
        (`MeshComponent.SetScalarParameterValueOnMaterials` (`self.Plane2`) "CustomTime" _output_get_2)
        (`MeshComponent.SetScalarParameterValueOnMaterials` (`self.Plane3`) "CustomTime" _output_get_2)
        (`MeshComponent.SetScalarParameterValueOnMaterials` (`self.Plane6`) "CustomTime" _output_get_2)
        (`MeshComponent.SetScalarParameterValueOnMaterials` (`self.Plane4`) "CustomTime" _output_get_2)
        (`MeshComponent.SetScalarParameterValueOnMaterials` (`self.Plane5`) "CustomTime" _output_get_2)
        (`SceneComponent.SetHiddenInGame` (`self.Cube2`) true false)
        (`SceneComponent.SetHiddenInGame` (`self.Cube3`) true false)
        (`SceneComponent.SetHiddenInGame` (`self.Cube4`) true false)
        (`SceneComponent.SetHiddenInGame` (`self.Cube5`) true false)
        (`SceneComponent.SetHiddenInGame` (`self.Cube`) true false)
        (`SceneComponent.SetHiddenInGame` (`self.Cube6`) true false)
        (`SceneComponent.SetHiddenInGame` (`self.Cube7`) true false)
        (`SceneComponent.SetHiddenInGame` (`self.Cube1`) true false)
        (`self.RollAlert`)
        (if (<= (`self.AlertCount`) 0)
          (goto _label :!via `Stop`)
          (else
            (set `self.AlertCount` 0)
            (goto _label)))))))

(event `self.ReceiveTick`
  (params (DeltaSeconds :type "Float (single-precision)")))

(event `ClearAlert`)

(event `RollAlert`
  (`SceneComponent.K2_AddWorldRotation` (`self.Center`) (struct :`Yaw` 25.0) false false))

(event `Spawn Orb`
  (`SceneComponent.SetHiddenInGame` (`self.BP_OrbObject`) false false)
  (`SceneComponent.SetHiddenInGame` (`self.BP_OrbObject1`) false false)
  (`SceneComponent.SetHiddenInGame` (`self.BP_OrbObject2`) false false))

(event `Roll_Reset`
  (`SceneComponent.K2_SetWorldRotation` :`self` (`self.Center`)))

(fn `UserConstructionScript`)