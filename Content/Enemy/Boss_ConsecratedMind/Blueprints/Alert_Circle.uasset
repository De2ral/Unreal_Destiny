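; Alert circle actor for the Consecrated Mind boss, likely an attack warning marker that removes itself when a tagged component reaches it.
; Its Sphere and Effect components both check overlapping components for a tag and destroy the actor on a match.
; Only the Effect overlap first spawns a large Energy_Charge Niagara burst at the Sphere's location.
; A timed self-destroy is unconnected, so only these overlaps remove it here.
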(event `self.ReceiveBeginPlay`)

(event `self.ReceiveTick`
  (params (DeltaSeconds :type "Float (single-precision)")))

(event `self.Sphere.OnComponentBeginOverlap`
  (params (OverlappedComponent :type "PrimitiveComponent Object Reference") (OtherActor :type "Actor Object Reference") (OtherComp :type "PrimitiveComponent Object Reference") (OtherBodyIndex :type Integer) (bFromSweep :type Boolean) (SweepResult :type "HitResult Structure (by ref)"))
  (if (`ActorComponent.ComponentHasTag` OtherComp (`self.Tag`))
    (`self.K2_DestroyActor`)))

(event `self.Effect.OnComponentBeginOverlap`
  (params (OverlappedComponent :type "PrimitiveComponent Object Reference") (OtherActor :type "Actor Object Reference") (OtherComp :type "PrimitiveComponent Object Reference") (OtherBodyIndex :type Integer) (bFromSweep :type Boolean) (SweepResult :type "HitResult Structure (by ref)"))
  (if (`ActorComponent.ComponentHasTag` OtherComp (`self.Tag`))
    (`NiagaraFunctionLibrary.SpawnSystemAtLocation` "/Game/Enemy/Dendron/FX/Energy_Charge.Energy_Charge" (`SceneComponent.K2_GetComponentLocation` (`self.Sphere`)) (struct) (20.0 20.0 20.0))
    (`self.K2_DestroyActor`)))

(fn `UserConstructionScript`)