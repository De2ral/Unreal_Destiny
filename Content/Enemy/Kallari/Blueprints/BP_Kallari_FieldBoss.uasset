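; Kallari field boss enemy with a camera-facing health bar, floating damage numbers and a melee hit volume.
; Attack events toggle the capsule's collision; overlapping a DestinyPlayer-tagged actor applies fixed damage, gated to one hit until shortly after overlap ends.
; AnyDamage sets RepNotify variables that update the health bar and spawn randomly offset damage-text actors, with doubled values for criticals.
; Death destroys both widget components.
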(event `self.ReceiveBeginPlay`
  (`PrimitiveComponent.SetCollisionEnabled` (`self.Capsule`) "NoCollision"))

(event `self.ReceiveTick`
  (params (DeltaSeconds :type "Float (single-precision)"))
  (bind _widget (`self.Widget`))
  (bind (_returnvalue_roll _returnvalue_pitch _returnvalue_yaw) (`KismetMathLibrary.BreakRotator` (`PlayerCameraManager.GetCameraRotation` (`GameplayStatics.GetPlayerCameraManager` 0))))
  (`/Engine/EditorBlueprintResources/StandardMacros.IsValid` _widget
    (:`Is Valid`
      (`SceneComponent.K2_SetWorldRotation` _widget (`KismetMathLibrary.MakeRotator` 0.0 0.0 (+ _returnvalue_yaw 180.0)) false false))))

(event `self.ReceiveAnyDamage`
  (params (Damage :type "Float (single-precision)") (DamageType :type "DamageType Object Reference") (InstigatedBy :type "Controller Object Reference") (DamageCauser :type "Actor Object Reference"))
  (if (`self.isDead`)
    (set `self.DamageText` Damage)
    (else
      (`self.RandomPosition`)
      (set `self.Progress_HP` (`self.HP`))
      (set `self.DamageText` Damage))))

(event `Dead_First`
  (bind _damage_widget (`self.Damage_Widget`))
  (bind _widget (`self.Widget`))
  (`/Engine/EditorBlueprintResources/StandardMacros.IsValid` _widget
    (:`Is Valid`
      (`ActorComponent.K2_DestroyComponent` _widget)
      (`/Engine/EditorBlueprintResources/StandardMacros.IsValid` _damage_widget
        (:`Is Valid`
          (`ActorComponent.K2_DestroyComponent` _damage_widget))))))

(event `Attack_Start`
  (`PrimitiveComponent.SetCollisionEnabled` (`self.Capsule`) "QueryAndPhysics"))

(event `Attack_End`
  (`PrimitiveComponent.SetCollisionEnabled` (`self.Capsule`) "NoCollision"))

(event `self.Capsule.OnComponentBeginOverlap`
  (params (OverlappedComponent :type "PrimitiveComponent Object Reference") (OtherActor :type "Actor Object Reference") (OtherComp :type "PrimitiveComponent Object Reference") (OtherBodyIndex :type Integer) (bFromSweep :type Boolean) (SweepResult :type "HitResult Structure (by ref)"))
  (if (`self.JustOneHit`)
    _
    (elif (`self.ActorHasTag` OtherActor "DestinyPlayer")
      (set `self.JustOneHit` true)
      (`GameplayStatics.ApplyDamage` OtherActor 20.0))))

(event `self.Capsule.OnComponentEndOverlap`
  (params (OverlappedComponent :type "PrimitiveComponent Object Reference") (OtherActor :type "Actor Object Reference") (OtherComp :type "PrimitiveComponent Object Reference") (OtherBodyIndex :type Integer))
  (if (`self.ActorHasTag` OtherActor "DestinyPlayer")
    (`KismetSystemLibrary.Delay` 0.2)
    (set `self.JustOneHit` false)))

(fn `OnRep_DamageText`
  (bind _damagetext (`self.DamageText`))
  (bind _returnvalue (`|SpawnActorFromClass` "/Game/Enemy/Dorongo/UI/DamageWidget_Actor.DamageWidget_Actor_C" (`KismetMathLibrary.MakeTransform` (`self.RandomDamagePoint`)) "Undefined" "OverrideRootScale" null null))
  (if (`self.bIsCriticalTextColor`)
    (`/Game/Enemy/Dorongo/UI/DamageWidget_Actor.SetDamageCriticalValue` _returnvalue (* _damagetext 2.0))
    (else
      (`/Game/Enemy/Dorongo/UI/DamageWidget_Actor.SetDamageValue` _returnvalue _damagetext)))
  (set `self.bIsCriticalTextColor` false))

(fn `OnRep_Progress_HP`
  (bind _asprogress_bar_kallari_field_boss (cast `/Game/Enemy/Kallari/UI/ProgressBar_Kallari_FieldBoss` (`WidgetComponent.GetWidget` (`self.Widget`))))
  (bind _progressbar (`/Game/Enemy/Kallari/UI/ProgressBar_Kallari_FieldBoss.ProgressBar` _asprogress_bar_kallari_field_boss)
    (:`then`
      (`ProgressBar.SetPercent` _progressbar (/ (`self.HP`) 10000.0)))
    (:`else`)))

(fn `RandomPosition`
  (bind _y (.y (`SceneComponent.K2_GetComponentLocation` (`self.WidgetPoint`))))
  (bind _z (.z (`SceneComponent.K2_GetComponentLocation` (`self.WidgetPoint`))))
  (set `self.RandomDamagePoint` (`KismetMathLibrary.MakeVector` (.x (`SceneComponent.K2_GetComponentLocation` (`self.WidgetPoint`))) (`KismetMathLibrary.RandomFloatInRange` (- _y 100.0) (+ _y 100.0)) (`KismetMathLibrary.RandomFloatInRange` (- _z 100.0) (+ _z 100.0)))))

(fn `UserConstructionScript`)