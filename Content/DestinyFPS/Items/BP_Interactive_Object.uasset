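; Base interactive object that flags itself interactive while an actor tagged DestinyPlayer is inside its sphere.
; Tick destroys it once HP reaches zero, and the Overlap RepNotify destroys it if it is interactive.
; The DestroyActor RepNotify instead runs chained custom events that teleport it far away and print "S" and "C" debug markers.
; HP, Overlap and the DestroyActor variable are not set in these graphs.
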(event `self.ReceiveActorBeginOverlap`
  (params (OtherActor :type "Actor Object Reference")))

(event `self.ReceiveTick`
  (params (DeltaSeconds :type "Float (single-precision)"))
  (if (<= (`self.HP`) 0.0)
    (`self.K2_DestroyActor`)))

(event `self.Sphere.OnComponentBeginOverlap`
  (params (OverlappedComponent :type "PrimitiveComponent Object Reference") (OtherActor :type "Actor Object Reference") (OtherComp :type "PrimitiveComponent Object Reference") (OtherBodyIndex :type Integer) (bFromSweep :type Boolean) (SweepResult :type "HitResult Structure (by ref)"))
  (if (`self.ActorHasTag` OtherActor "DestinyPlayer")
    (set `self.IsInteractive` true)))

(event `self.Sphere.OnComponentEndOverlap`
  (params (OverlappedComponent :type "PrimitiveComponent Object Reference") (OtherActor :type "Actor Object Reference") (OtherComp :type "PrimitiveComponent Object Reference") (OtherBodyIndex :type Integer))
  (if (`self.ActorHasTag` OtherActor "DestinyPlayer")
    (set `self.IsInteractive` false)))

(event `커스텀이벤트`
  (`self.K2_SetActorLocation` (0.0 111111111.0 0.0) false true)
  (`self.커스텀이벤트_0`)
  (`KismetSystemLibrary.PrintString` "S"))

(event `커스텀이벤트_0`
  (`self.K2_SetActorLocation` (0.0 111111111.0 0.0) false true)
  (`KismetSystemLibrary.PrintString` "C"))

(fn `OnRep_DestroyActor`
  (`self.커스텀이벤트`))

(fn `OnRep_IsInteractive`)

(fn `OnRep_Overlap`
  (if (`self.IsInteractive`)
    (`self.K2_DestroyActor`)))

(fn `UserConstructionScript`)